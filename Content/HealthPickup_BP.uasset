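; HealthPickup_BP is a pickup actor that restores health to the first-person character.
; When its Sphere component begins overlapping a FirstPersonCharacter below max health, it fires the OnCorrectCollision dispatcher with HealthToAdd, passes that amount to the character's AdjustHealth, then destroys itself.
; At full health the pickup stays in place, and other overlapping actors only print a cast failure message.
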(event `self.Sphere.OnComponentBeginOverlap`
  (params (OverlappedComponent :type "PrimitiveComponent Object Reference") (OtherActor :type "Actor Object Reference") (OtherComp :type "PrimitiveComponent Object Reference") (OtherBodyIndex :type Integer) (bFromSweep :type Boolean) (SweepResult :type "HitResult Structure (by ref)"))
  (bind _healthtoadd (`self.HealthToAdd`))
  (bind _asfirst_person_character (cast `/Game/FirstPersonCPP/Blueprints/FirstPersonCharacter` OtherActor)
    (:`then`
      (if (< (`/Game/FirstPersonCPP/Blueprints/FirstPersonCharacter.Health` _asfirst_person_character) (`/Game/FirstPersonCPP/Blueprints/FirstPersonCharacter.MaxHealth` _asfirst_person_character))
        (if true
          (`self.onCorrectCollision` _healthtoadd))
        (`/Game/FirstPersonCPP/Blueprints/FirstPersonCharacter.AdjustHealth` _asfirst_person_character _healthtoadd)
        (`self.K2_DestroyActor`)))
    (:`CastFailed`
      (`KismetSystemLibrary.PrintString` "CastFailed"))))

(fn `UserConstructionScript`)