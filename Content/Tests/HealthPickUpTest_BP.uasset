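; Functional test for health pickups that checks whether a referenced actor's health is correct after collecting one.
; PrepareTest binds to existing pickups' collision events and the actor's GotHealth event.
; Collision computes expected health capped at MaxHealth, and GotHealth passes or fails the test on an exact match.
; Tick also spawns items at intervals, without binding them, and reports success two seconds after the last spawn.
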(event `self.ReceiveTick`
  (params (DeltaSeconds :type "Float (single-precision)"))
  (bind _output_get (set `self.Timer` (+ DeltaSeconds (`self.Timer`))))
  (if (and (>= _output_get (`self.spawnInterval`)) (> (`self.ItemsToSpawn`) 0))
    (`self.SpawnItem`)
    (set `self.Timer` 0.0)
    (bind _result (`/Engine/EditorBlueprintResources/StandardMacros.DecrementInt` (`self.ItemsToSpawn`))
      (:`  `
        (if (<= _result 0)
          (`KismetSystemLibrary.Delay` 2.0)
          (`self.FinishTest` "Succeeded"))))))

(event `self.ReceivePrepareTest`
  (bind _outactors (`GameplayStatics.GetAllActorsOfClass` (`self.Class`)))
  (for _array_element _outactors
    (add `/Game/HealthPickup_BP.onCorrectCollision` _array_element (delegate `CustomEvent_0`))
    (add `/Game/FirstPersonCPP/Blueprints/FirstPersonCharacter.GotHealth` (`self.NewVar_0`) (delegate `CustomEvent_1`))))

(event `CustomEvent_0`
  (params (Health :type Integer))
  (bind _newvar_0 (`self.NewVar_0`))
  (bind _maxhealth (`/Game/FirstPersonCPP/Blueprints/FirstPersonCharacter.MaxHealth` _newvar_0))
  (bind _returnvalue (+ Health (`/Game/FirstPersonCPP/Blueprints/FirstPersonCharacter.Health` _newvar_0)))
  (`KismetSystemLibrary.PrintString` "Hello")
  (if (> _returnvalue _maxhealth)
    (bind _output_get (set `self.ExpectedHealth` _maxhealth))
    (else
      (set `self.ExpectedHealth` _returnvalue)))
  (set `self.NewVar_2` (`KismetMathLibrary.Conv_IntToBool` _output_get)))

(event `CustomEvent_1`
  (params (CurrentHealth :type Integer))
  (if (== CurrentHealth (`self.ExpectedHealth`))
    (`KismetSystemLibrary.PrintString` "win")
    (`self.FinishTest` "Succeeded")
    (else
      (`KismetSystemLibrary.PrintString` "fail")
      (`self.FinishTest` "Failed"))))

(fn `SpawnItem`
  (`|SpawnActorFromClass` (`self.Class`) (`self.GetTransform`) "Undefined" "OverrideRootScale" null null))

(fn `TEst`)

(fn `UserConstructionScript`)